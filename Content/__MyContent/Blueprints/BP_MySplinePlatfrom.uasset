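; Platform actor that moves a mesh along a spline, starting at BeginPlay.
; A timeline curve scales the spline length into a distance, and each update sets the mesh's world location at that point without sweeping or changing rotation.
; When the timeline finishes, it replays from the start if Loop is enabled.
; The construction script applies the configurable static mesh and material to the platform.
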(event Custom|PlatformStart
  (bind _spline (Variables|Default|GetSpline))
  (bind _sline_distance (Timeline|Motion%20timeline PlayFromStart)
    (:Update
      (Transformation|SetWorldLocation (Variables|Default|GetPlatform%20Mesh) (Spline|GetLocationatDistanceAlongSpline _spline (* _sline_distance (Spline|GetSplineLength _spline)) "World") false false))
    (:Finished
      (if (Variables|Default|GetLoop)
        (CallFunction|PlatformStart)))))

(event EventBeginPlay
  (CallFunction|PlatformStart))

(fn ConstructionScript
  (bind _platform_mesh (Variables|Default|GetPlatform%20Mesh))
  (Components|StaticMesh|SetStaticMesh _platform_mesh (Variables|Default|GetStatic%20Mesh))
  (Rendering|Material|SetMaterial _platform_mesh 0 (Variables|Default|GetMaterial)))