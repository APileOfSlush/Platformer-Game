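; Waypoint-driven moving platform with a configurable mesh and material, which hides its waypoint actors on BeginPlay and starts moving.
; MotionTimeline, played at Rate, lerps the actor's relative location between the current and next waypoints' world positions.
; Its event track advances the waypoint index, or at path end jumps back to the first segment if Loop is set.
; Start and Stop functions control the motion.
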(event Custom|platform%20start
  (bind _motion_timeline (Variables|Default|Getmotion%20timeline))
  (CallFunction|SetFirstWaypoint)
  (Components|Timeline|SetPlayRate _motion_timeline (Variables|Default|GetRate))
  (Components|Timeline|PlayfromStart _motion_timeline))

(event EventBeginPlay
  (for _array_element (Variables|Default|Getwaypoints)
    (Rendering|SetActorHiddenInGame _array_element true)
    (CallFunction|PlatformStart)))

(fn ConstructionScript
  (bind _platform_mesh (Variables|Default|GetPlatform%20mesh))
  (Components|StaticMesh|SetStaticMesh _platform_mesh (Variables|Default|GetStaticMesh))
  (Rendering|Material|SetMaterial _platform_mesh 0 (Variables|Default|GetMaterial)))

(fn SetPositions
  (bind _waypoints (Variables|Default|Getwaypoints))
  (Variables|Default|SetCurrent%20Waypoint%20position (Transformation|GetActorLocation (Utilities|Array|Get(acopy) _waypoints (Variables|Default|GetCurrent%20waypoint%20index))))
  (Variables|Default|SetNext%20waypoint%20position (Transformation|GetActorLocation (Utilities|Array|Get(acopy) _waypoints (Variables|Default|GetNext%20waypoint%20index)))))

(fn SetFirstWaypoint
  (Variables|Default|SetCurrent%20waypoint%20index 0)
  (Variables|Default|SetNext%20waypoint%20index 1)
  (CallFunction|SetPositions))

(fn SetNextWaypoint
  (bind _result (Math|Integer|IncrementInt (Variables|Default|GetCurrent%20waypoint%20index))
    (:%20%20
      (Variables|Default|SetNext%20waypoint%20index (+ _result 1))
      (CallFunction|SetPositions))))

(fn PathIsFinished
  (return (== (Variables|Default|GetNext%20waypoint%20index) (- (Utilities|Array|Length (Variables|Default|Getwaypoints)) 1))))

(fn Start
  (CallFunction|PlatformStart))

(fn Stop
  (Audio|Components|Audio|Stop (Variables|Default|Getmotion%20timeline)))