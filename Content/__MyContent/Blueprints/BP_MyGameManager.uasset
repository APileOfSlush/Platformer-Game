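; Game manager Blueprint that controls the overall game state: Running, Win, Lose or Abandon.
; Init has BP_MyGamemode create the UI, initializes the player, then enters Running.
; SetState acts only on changes, hiding UI, then either showing the HUD and unpausing, or showing that outcome's widget with mouse cursor and pause.
; ResetGame only re-initializes the player; its PlayerStart teleport and level-reload nodes are disconnected.
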(event EventBeginPlay)

(event Collision|EventActorBeginOverlap
  (params (OtherActor :type Actor%20Object%20Reference)))

(event EventTick
  (params (DeltaSeconds :type Float%20%28single-precision%29)))

(fn ConstructionScript)

(fn Init
  (bind _asbp_my_gamemode (Utilities|Casting|CastToBP_MyGamemode (Game|GetGameMode)))
  (Default|CreateUI _asbp_my_gamemode)
  (Default|Init (Variables|Default|GetMy%20Player))
  (CallFunction|SetState "NewEnumerator0"))

(fn SetState
  (params (New%20State :type E_MyGameStates%20Enum :default "NewEnumerator0"))
  (if (Utilities|Enum|NotEqual(Enum) New%20State (Variables|Default|GetCurrent%20Game%20State))
    (CallFunction|HideUI)
    (bind _output_get (Variables|Default|SetCurrent%20Game%20State New%20State))
    (switch Utilities|FlowControl|Switch|SwitchonE_MyGameStates _output_get
      (:NewEnumerator0
        (CallFunction|ShowMouse false)
        (CallFunction|ShowHud true)
        (Game|SetGamePaused false))
      (:NewEnumerator1
        (Widget|SetVisibility (Variables|Default|GetWIdget_Win) "Visible")
        (Game|SetGamePaused true :!label _label)
        (CallFunction|ShowMouse true))
      (:NewEnumerator2
        (Widget|SetVisibility (Variables|Default|GetWidget_Lose) "Visible")
        (goto _label))
      (:NewEnumerator3
        (Widget|SetVisibility (Variables|Default|GetWIdget_Abandon) "Visible")
        (goto _label)))))

(fn GetState
  (return (Variables|Default|GetCurrent%20Game%20State)))

(fn ResetGame
  (Default|Init (Variables|Default|GetMy%20Player)))

(fn ShowHud
  (params (Visible :type Boolean))
  (bind _widget_health (Variables|Default|GetWidget_Health))
  (if Visible
    (Widget|SetVisibility _widget_health "Visible")
    (else
      (Widget|SetVisibility _widget_health "Hidden"))))