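; BP_MyGamemode is a game mode Blueprint that locates the game manager and builds the player's UI.
; On BeginPlay it caches the first BP_MyGameManager actor found in the level.
; CreateUI creates the abandon, win, lose, health, minimap and stamina widgets, stores each reference on that manager and adds all of them to the viewport.
; Nothing in this Blueprint calls CreateUI itself.
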(event EventBeginPlay
  (bind _outactors (Actor|GetAllActorsOfClass "/Game/__MyContent/Blueprints/BP_MyGameManager.BP_MyGameManager_C"))
  (Variables|Default|SetMy%20Game%20manager (Utilities|Array|Get(acopy) _outactors)))

(fn ConstructionScript)

(fn CreateUI
  (bind _my_game_manager (Variables|Default|GetMy%20Game%20manager))
  (bind _returnvalue (UserInterface|CreateWidget "/Game/__MyContent/UI/Widget_Abandon.Widget_Abandon_C"))
  (bind _output_get (Variables|/Game/__MyContent/Blueprints/BP_MyGameManager.BP_MyGameManager_C|SetWIdget_Abandon _my_game_manager _returnvalue))
  (UserInterface|Viewport|AddtoViewport _output_get 0)
  (bind _returnvalue_2 (UserInterface|CreateWidget "/Game/__MyContent/UI/Widget_WIn.Widget_WIn_C"))
  (bind _output_get_2 (Variables|/Game/__MyContent/Blueprints/BP_MyGameManager.BP_MyGameManager_C|SetWIdget_Win _my_game_manager _returnvalue_2))
  (UserInterface|Viewport|AddtoViewport _output_get_2 0)
  (bind _returnvalue_3 (UserInterface|CreateWidget "/Game/__MyContent/UI/WIdget_Lose.WIdget_Lose_C"))
  (bind _output_get_3 (Variables|/Game/__MyContent/Blueprints/BP_MyGameManager.BP_MyGameManager_C|SetWidget_Lose _my_game_manager _returnvalue_3))
  (UserInterface|Viewport|AddtoViewport _output_get_3 0)
  (bind _returnvalue_4 (UserInterface|CreateWidget "/Game/__MyContent/UI/Widget_health.Widget_health_C"))
  (bind _output_get_4 (Variables|/Game/__MyContent/Blueprints/BP_MyGameManager.BP_MyGameManager_C|SetWidget_Health _my_game_manager _returnvalue_4))
  (UserInterface|Viewport|AddtoViewport _output_get_4 0)
  (bind _returnvalue_5 (UserInterface|CreateWidget "/Game/__MyContent/UI/Widget_MiniMap.Widget_MiniMap_C"))
  (bind _output_get_5 (Variables|/Game/__MyContent/Blueprints/BP_MyGameManager.BP_MyGameManager_C|SetWidget_Minimap _my_game_manager _returnvalue_5))
  (UserInterface|Viewport|AddtoViewport _output_get_5 0)
  (bind _returnvalue_6 (UserInterface|CreateWidget "/Game/__MyContent/UI/Widget_Stamina.Widget_Stamina_C"))
  (bind _output_get_6 (Variables|/Game/__MyContent/Blueprints/BP_MyGameManager.BP_MyGameManager_C|SetWidget_Stamina _my_game_manager _returnvalue_6))
  (UserInterface|Viewport|AddtoViewport _output_get_6 0))